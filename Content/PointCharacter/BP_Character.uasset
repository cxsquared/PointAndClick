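; Player character Blueprint that shows timed speech text in a screen widget following the player.
; BeginPlay creates a hidden WB_PlayerText widget and adds it to the viewport.
; Talk sets and shows the text, restarting a name-based timer that calls ClearText to empty and hide it.
; Every Tick, UpdateText projects player 0's capsule location to screen space and positions the widget there with a fixed offset.
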(event `self.ReceiveBeginPlay`
  (bind _returnvalue (`|CreateWidget` "/Game/PointClick/UI/WB_PlayerText.WB_PlayerText_C"))
  (bind _output_get (set `self.Widget` _returnvalue))
  (`UserWidget.AddToViewport` _output_get 0)
  (`Widget.SetVisibility` _output_get "Hidden")
  (`UserWidget.SetDesiredSizeInViewport` _output_get (500.0 200.0)))

(event `self.ReceiveActorBeginOverlap`
  (params (OtherActor :type "Actor Object Reference")))

(event `self.ReceiveTick`
  (params (DeltaSeconds :type "Float (single-precision)"))
  (`self.UpdateText`))

(fn `ClearText`
  (`/Game/PointClick/UI/WB_PlayerText.SetText` (`self.Widget`) "")
  (`KismetSystemLibrary.K2_ClearTimer` null "ClearText")
  (`Widget.SetVisibility` (`self.Widget`) "Hidden"))

(fn `Talk`
  (params (Text :type String) (DisplayTime :type "Float (double-precision)"))
  (`/Game/PointClick/UI/WB_PlayerText.SetText` (`self.Widget`) Text)
  (`KismetSystemLibrary.K2_ClearTimer` null "ClearText")
  (`KismetSystemLibrary.K2_SetTimer` null "ClearText" DisplayTime)
  (`Widget.SetVisibility` (`self.Widget`) "Visible"))

(fn `UpdateText`
  (`UserWidget.SetPositionInViewport` (`self.Widget`) (- (`WidgetLayoutLibrary.ProjectWorldLocationToWidgetPosition` (`GameplayStatics.GetPlayerController` 0) (`SceneComponent.K2_GetComponentLocation` (`Character.CapsuleComponent` (`GameplayStatics.GetPlayerCharacter` 0)))) (250.0 200.0)) false)
  (return))

(fn `UserConstructionScript`)