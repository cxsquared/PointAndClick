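; Point-and-click camera actor that slowly turns its camera component to follow the player character.
; Each Tick, while the player controller (PC_PointCharacter) has CanCameraMove set, it interpolates the forward vector toward the unnormalized camera-to-player offset at very low speed.
; The result sets world pitch and yaw with zero roll.
; The angle clamps are centered on that same result, so they never limit rotation.
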(event `self.ReceiveBeginPlay`)

(event `self.ReceiveActorBeginOverlap`
  (params (OtherActor :type "Actor Object Reference")))

(event `self.ReceiveTick`
  (params (DeltaSeconds :type "Float (single-precision)"))
  (bind _camera (`self.Camera`))
  (bind _pitch (.pitch (`KismetMathLibrary.Conv_VectorToRotator` (`KismetMathLibrary.VInterpTo` (`KismetMathLibrary.Conv_RotatorToVector` (`SceneComponent.K2_GetComponentRotation` _camera)) (- (`self.K2_GetActorLocation` (`GameplayStatics.GetPlayerCharacter` 0)) (`SceneComponent.K2_GetComponentLocation` _camera)) (`self.DT_DeltaTime`) 0.001))))
  (bind _yaw (.yaw (`KismetMathLibrary.Conv_VectorToRotator` (`KismetMathLibrary.VInterpTo` (`KismetMathLibrary.Conv_RotatorToVector` (`SceneComponent.K2_GetComponentRotation` _camera)) (- (`self.K2_GetActorLocation` (`GameplayStatics.GetPlayerCharacter` 0)) (`SceneComponent.K2_GetComponentLocation` _camera)) (`self.DT_DeltaTime`) 0.001))))
  (set `self.DT_DeltaTime` DeltaSeconds)
  (bind _aspc_point_character (cast `/Game/PointClick/Blueprint/PC_PointCharacter` (`GameplayStatics.GetPlayerController` 0)))
  (if (`/Game/PointClick/Blueprint/PC_PointCharacter.CanCameraMove` _aspc_point_character)
    (`SceneComponent.K2_SetWorldRotation` _camera (`KismetMathLibrary.MakeRot` (`KismetMathLibrary.ClampAngle` _pitch (- _pitch 80.0) (+ _pitch 80.0)) (`KismetMathLibrary.ClampAngle` _yaw (- _yaw 80.0) (+ _yaw 80.0))) true)))

(fn `UserConstructionScript`)