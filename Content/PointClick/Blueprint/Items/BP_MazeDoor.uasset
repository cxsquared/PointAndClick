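; BP_MazeDoor is an interactable maze door that records the player's completion of the maze room and starts a teleport.
; The first Interact increments RoomsComplete on BP_Character, flags DidMaze and copies the door's IsRed value into PickedRed.
; A DoOnce guards that bookkeeping, while a Sequence still calls StartTeleport on every interaction.
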(event `self.ReceiveBeginPlay`)

(event `self.ReceiveActorBeginOverlap`
  (params (OtherActor :type "Actor Object Reference")))

(event `self.ReceiveTick`
  (params (DeltaSeconds :type "Float (single-precision)"))
  (`parent.ReceiveTick` 0.0))

(event `/Game/PointClick/Blueprint/Items/BP_Pickup.Interact`
  (`|ExecutionSequence`
    (:`then_0`
      (`/Engine/EditorBlueprintResources/StandardMacros.DoOnce` false
        (:`Completed`
          (bind _asbp_character (cast `/Game/PointCharacter/BP_Character` (`GameplayStatics.GetPlayerCharacter` 0)))
          (set `/Game/PointCharacter/BP_Character.RoomsComplete` (+ (`/Game/PointCharacter/BP_Character.RoomsComplete` _asbp_character) 1) _asbp_character)
          (set `/Game/PointCharacter/BP_Character.DidMaze` true _asbp_character)
          (set `/Game/PointCharacter/BP_Character.PickedRed` (`self.IsRed`) _asbp_character))))
    (:`then_1`
      (`/Game/PointClick/Blueprint/Items/BP_LevelDoor.StartTeleport`))))

(fn `UserConstructionScript`
  (`parent.UserConstructionScript`))