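; BP_DoorItem is an interactable locked door for a point-and-click game that requires a "Key" item to open.
; On Interact, it asks the player controller PC_PointCharacter for the key.
; If found, it removes the key, disables the Item component's collision and destroys the door actor.
; Otherwise, the player character says a short line about lacking the key.
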(event `self.ReceiveBeginPlay`)

(event `self.ReceiveActorBeginOverlap`
  (params (OtherActor :type "Actor Object Reference")))

(event `self.ReceiveTick`
  (params (DeltaSeconds :type "Float (single-precision)"))
  (`parent.ReceiveTick` 0.0))

(event `self.Interact`
  (bind _aspc_point_character (cast `/Game/PointClick/Blueprint/PC_PointCharacter` (`GameplayStatics.GetPlayerController` 0)))
  (bind _item (`/Game/PointClick/Blueprint/PC_PointCharacter.GetItem` _aspc_point_character "Key"))
  (if (`KismetStringLibrary.NotEqual_StrStr` (`.Name_2_34A361EA46F0130E44C349B8924FD24E` (break `/Game/PointClick/Blueprint/Struct_Item` _item)) "null")
    (bind _aspc_point_character_2 (cast `/Game/PointClick/Blueprint/PC_PointCharacter` (`GameplayStatics.GetPlayerController` 0)))
    (`/Game/PointClick/Blueprint/PC_PointCharacter.RemoveItem` _aspc_point_character_2 _item)
    (`PrimitiveComponent.SetCollisionEnabled` (`self.Item`) "NoCollision")
    (`self.K2_DestroyActor`)
    (else
      (bind _asbp_character (cast `/Game/Character/BP_Character` (`GameplayStatics.GetPlayerCharacter` 0)))
      (`/Game/Character/BP_Character.Talk` _asbp_character "I don't have the key" 5.0))))

(fn `UserConstructionScript`
  (`parent.UserConstructionScript`))