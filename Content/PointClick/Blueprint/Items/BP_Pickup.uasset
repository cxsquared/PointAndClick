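; Point-and-click pickup item that the player can examine or collect into the inventory held by PC_PointCharacter.
; Pressing it shows an interaction widget; releasing left of the press speaks its description, otherwise the character walks to it.
; A looping WalkTo timer checks distance, then Interact adds the item and hides it, while another left click cancels the approach.
; Use only gives a doesn't-work line, and the per-tick UpdateMenu is empty.
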(event OnClicked(Box)
  (params (TouchedComponent :type Primitive%20Component%20Object%20Reference))
  (bind _returnvalue (Game|GetPlayerController 0))
  (bind _aspc_point_character (Utilities|Casting|CastToPC_PointCharacter _returnvalue))
  (if (Variables|/Game/PointClick/Blueprint/PC_PointCharacter.PC_PointCharacter_C|GetCanInteract _aspc_point_character)
    (if (not (Variables|Default|GetIsClicked))
      (Variables|Default|SetIsClicked true)
      (Variables|Default|SetFirstTouch (.LocationX (Game|Player|GetMousePosition _returnvalue)))
      (bind _returnvalue_2 (UserInterface|CreateWidget "/Game/PointClick/UI/WB_Interaction.WB_Interaction_C"))
      (bind _output_get (Variables|Default|SetWidget _returnvalue_2))
      (Class|Widget|SetRenderTranslation _output_get (.ScreenPosition (Class|WidgetLayoutLibrary|ProjectWorldLocationtoWidgetPosition (Game|GetPlayerController 0) (Transformation|GetWorldLocation (Variables|Default|GetItem)))))
      (UserInterface|Viewport|AddtoViewport _output_get 0))))

(event OnReleased(Box)
  (params (TouchedComponent :type Primitive%20Component%20Object%20Reference))
  (if (Variables|Default|GetIsClicked)
    (Variables|Default|SetIsClicked false)
    (Widget|RemovefromParent (Variables|Default|GetWidget))
    (if (> (Variables|Default|GetFirstTouch) (.LocationX (Game|Player|GetMousePosition (Game|GetPlayerController 0))))
      (CallFunction|Look)
      (else
        (Variables|Default|SetIsInteracting true)
        (CallFunction|Walkto)))))

(event OnEndCursorOver(Box)
  (params (TouchedComponent :type Primitive%20Component%20Object%20Reference))
  (Variables|Default|SetIsClicked false)
  (Widget|RemovefromParent (Variables|Default|GetWidget)))

(event EventBeginPlay)

(event Collision|EventActorBeginOverlap
  (params (OtherActor :type Actor%20Object%20Reference)))

(event EventTick
  (params (DeltaSeconds :type Float%20%28single-precision%29))
  (CallFunction|UpdateMenu))

(event Input|ActionEvents|InputActionLeftMouseClick
  ;[1 1 1] Comment
  (:Pressed
    (if (and (Variables|Default|GetIsInteracting) (Variables|Default|GetPlayerApproching))
      (Variables|Default|SetIsInteracting false)
      (Variables|Default|SetPlayerApproching false)
      (Utilities|Time|ClearTimerbyFunctionName 0 "WalkTo"))))

(fn ConstructionScript)

(fn Interact
  (if (Variables|Default|GetCanBePickedUp)
    (bind _aspc_point_character (Utilities|Casting|CastToPC_PointCharacter (Game|GetPlayerController 0)))
    (Default|AddItem _aspc_point_character (stale _output_get))
    (Rendering|SetVisibility (Variables|Default|GetItem) false true)
    (Collision|SetCollisionEnabled (Variables|Default|GetBox) "NoCollision")))

(fn Look
  (bind _asbp_character (Utilities|Casting|CastToBP_Character (Game|GetPlayerCharacter 0)))
  (Default|Talk _asbp_character (.Description (Utilities|Struct|BreakStruct_Item (Variables|Default|GetItemStruct))) 5.0))

(fn UpdateMenu)

(fn Use
  (params (UsingItem :type BP%20Pickup%20Object%20Reference))
  (if (not false)
    (bind _asbp_character (Utilities|Casting|CastToBP_Character (Game|GetPlayerCharacter 0)))
    (Default|Talk _asbp_character "I don't think it works with that." 5.0)))

(fn Walkto
  (bind _self self)
  (if (Variables|Default|GetIsInteracting)
    (if (<= (Transformation|GetDistanceTo (Game|GetPlayerCharacter 0) self) 2e+02)
      (Variables|Default|SetIsInteracting false)
      (Variables|Default|SetPlayerApproching false)
      (Utilities|Time|ClearTimerbyFunctionName 0 "WalkTo")
      (CallFunction|Interact)
      (goto _label Reset)
      (else
        (Utilities|FlowControl|DoOnce false :!label _label
          (:Completed
            (AI|Navigation|SimpleMovetoActor 0 _self)
            (Utilities|Time|SetTimerbyFunctionName _self "WalkTo" 0.1 true)
            (Variables|Default|SetPlayerApproching true)))))))