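; BP_LevelDoor is an interactable point-and-click door that moves the player to another room's spawn point.
; Interact checks CanTeleport and a non-zero RoomSpawn location, otherwise the character says it won't open; Look gives a remark.
; A valid use plays a fade-out and sound, flags talking rooms on PC_PointCharacter, and stops movement.
; A two-second timer then teleports the player to RoomSpawn and fades in.
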(event `self.ReceiveBeginPlay`)

(event `self.ReceiveActorBeginOverlap`
  (params (OtherActor :type "Actor Object Reference")))

(event `self.ReceiveTick`
  (params (DeltaSeconds :type "Float (single-precision)"))
  (`parent.ReceiveTick` 0.0))

(event `/Game/PointClick/Blueprint/Items/BP_Pickup.Interact`
  (bind _returnvalue (`GameplayStatics.GetPlayerController` 0))
  (if (`self.CanTeleport`)
    (if (!= (`.Location_2_5192FD9B4532D4A06560AC906EC84ACA` (break `/Game/PointClick/Blueprint/Struct_TeleportDest` (`self.RoomSpawn`))) (0.0 0.0 0.0))
      (`self.StartTeleport`)
      (if (`.TalkingRoom_8_AB158B9A47F9CEFE66464AA54485CE4F` (break `/Game/PointClick/Blueprint/Struct_TeleportDest` (`self.RoomSpawn`)))
        (bind _aspc_point_character (cast `/Game/PointClick/Blueprint/PC_PointCharacter` _returnvalue))
        (set `/Game/PointClick/Blueprint/PC_PointCharacter.InTalkingRoom` true _aspc_point_character))
      (`Controller.StopMovement` _returnvalue)
      (else
        (bind _asbp_character (cast `/Game/PointCharacter/BP_Character` (`GameplayStatics.GetPlayerCharacter` 0) :!label _label))
        (`/Game/PointCharacter/BP_Character.Talk` _asbp_character "It won't open" 5.0)))
    (else
      (goto _label))))

(event `/Game/PointClick/Blueprint/Items/BP_Pickup.Look`
  (bind _asbp_character (cast `/Game/PointCharacter/BP_Character` (`GameplayStatics.GetPlayerCharacter` 0)))
  (`/Game/PointCharacter/BP_Character.Talk` _asbp_character "I wonder where it leads?" 5.0))

(fn `StartTeleport`
  (bind _fadeout (`self.FadeOut`))
  (`MatineeActor.SetPosition` _fadeout 0.0 true)
  (`MatineeActor.Play` _fadeout)
  (bind _returnvalue (`AddComponent|Audio Component_1`))
  (`AudioComponent.Play` _returnvalue 0.0)
  (`KismetSystemLibrary.K2_SetTimer` null "Teleport" 2.0))

(fn `Teleport`
  (bind (_location _rotation) (break `/Game/PointClick/Blueprint/Struct_TeleportDest` (`self.RoomSpawn`)))
  (`self.K2_TeleportTo` (`GameplayStatics.GetPlayerCharacter` 0) _location _rotation)
  (`MatineeActor.Play` (`self.FadeIn`))
  (return))

(fn `UserConstructionScript`
  (`parent.UserConstructionScript`))