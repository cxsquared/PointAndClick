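; A return door actor that sends the player character back to a linked return spawn point in a point-and-click game.
; Its Teleport event plays a FadeOut, moves the player to the location and rotation in ReturnSpawn's SpawnData, stops controller movement, then plays a FadeIn.
; BeginPlay, overlap and Tick are unused, so teleporting runs only when the Teleport event is invoked.
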(event `self.ReceiveBeginPlay`)

(event `self.ReceiveActorBeginOverlap`
  (params (OtherActor :type "Actor Object Reference")))

(event `self.ReceiveTick`
  (params (DeltaSeconds :type "Float (single-precision)"))
  (`parent.ReceiveTick` 0.0))

(event `self.Teleport`
  (bind (_location _rotation) (break `/Game/PointClick/Blueprint/Struct_TeleportDest` (`/Game/PointClick/Blueprint/BP_SpawnLocation.SpawnData` (`self.ReturnSpawn`))))
  (`MatineeActor.Play` (`self.FadeOut`))
  (`self.K2_TeleportTo` (`GameplayStatics.GetPlayerCharacter` 0) _location _rotation)
  (`Controller.StopMovement` (`GameplayStatics.GetPlayerController` 0))
  (`MatineeActor.Play` (`self.FadeIn`)))

(fn `UserConstructionScript`
  (`parent.UserConstructionScript`))