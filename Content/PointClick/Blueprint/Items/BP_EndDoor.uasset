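; BP_EndDoor is an interactable exit door that ends a point-and-click game once enough rooms are finished.
; On Interact it casts the player character to BP_Character and checks its RoomsComplete count against a threshold of two.
; If met, the character speaks a farewell line and, after a matching delay, the Start level opens; otherwise the character says the door is stuck.
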(event `self.ReceiveBeginPlay`)

(event `self.ReceiveActorBeginOverlap`
  (params (OtherActor :type "Actor Object Reference")))

(event `self.ReceiveTick`
  (params (DeltaSeconds :type "Float (single-precision)"))
  (`parent.ReceiveTick` 0.0))

(event `/Game/PointClick/Blueprint/Items/BP_Pickup.Interact`
  (bind _asbp_character (cast `/Game/PointCharacter/BP_Character` (`GameplayStatics.GetPlayerCharacter` 0)))
  (if (>= (`/Game/PointCharacter/BP_Character.RoomsComplete` _asbp_character) 2)
    (`/Game/PointCharacter/BP_Character.Talk` _asbp_character "Looks like I can get out of here. Thank you I think." 3.0)
    (`KismetSystemLibrary.Delay` 3.0)
    (`GameplayStatics.OpenLevel` "Start")
    (else
      (`/Game/PointCharacter/BP_Character.Talk` _asbp_character "It won't open. Let's check the other doors." 3.0))))

(fn `UserConstructionScript`
  (`parent.UserConstructionScript`))