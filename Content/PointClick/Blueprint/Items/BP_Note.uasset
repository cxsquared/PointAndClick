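; BP_Note is a point-and-click item that has the player character read out a randomly chosen note.
; BeginPlay picks one note from NoteOptions, and both Look and Interact lock the controller's movement and interaction, then start it.
; ShowNoteEvent calls itself after each line's duration, using ShowNote to send text to BP_Character's Talk.
; Control returns after the last line is sent, without waiting out its duration.
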(event Custom|ShowNoteEvent
  (params (Line :type Integer))
  (bind _aspc_point_character (Utilities|Casting|CastToPC_PointCharacter (Game|GetPlayerController 0)))
  (Variables|/Game/PointClick/Blueprint/PC_PointCharacter.PC_PointCharacter_C|SetCanInteract _aspc_point_character false)
  (Variables|/Game/PointClick/Blueprint/PC_PointCharacter.PC_PointCharacter_C|SetCanMove _aspc_point_character false)
  (bind (_nextline _nextdelaytime) (CallFunction|ShowNote Line))
  (if (> _nextline 0)
    (if (< _nextline (Utilities|Array|Length (Utilities|Struct|BreakStruct_Note (Variables|Default|GetNote))))
      (Utilities|FlowControl|Delay _nextdelaytime)
      (CallFunction|ShowNoteEvent _nextline)
      (else
        (bind _aspc_point_character_2 (Utilities|Casting|CastToPC_PointCharacter (Game|GetPlayerController 0)))
        (Variables|/Game/PointClick/Blueprint/PC_PointCharacter.PC_PointCharacter_C|SetCanMove _aspc_point_character_2 true)
        (Variables|/Game/PointClick/Blueprint/PC_PointCharacter.PC_PointCharacter_C|SetCanInteract _aspc_point_character_2 true)))))

(event EventInteract
  (bind _aspc_point_character (Utilities|Casting|CastToPC_PointCharacter (Game|GetPlayerController 0)))
  (Variables|/Game/PointClick/Blueprint/PC_PointCharacter.PC_PointCharacter_C|SetCanInteract _aspc_point_character false)
  (Variables|/Game/PointClick/Blueprint/PC_PointCharacter.PC_PointCharacter_C|SetCanMove _aspc_point_character false)
  (CallFunction|ShowNoteEvent))

(event EventBeginPlay
  (bind _noteoptions (Variables|Default|GetNoteOptions))
  (Variables|Default|SetNote (Utilities|Array|Get(acopy) _noteoptions (Math|Random|RandomIntegerinRange 0 (- (Utilities|Array|Length _noteoptions) 1)))))

(event Collision|EventActorBeginOverlap
  (params (OtherActor :type Actor%20Object%20Reference)))

(event EventTick
  (params (DeltaSeconds :type Float%20%28single-precision%29))
  (|CallParentFunction 0.0))

(event EventLook
  (bind _aspc_point_character (Utilities|Casting|CastToPC_PointCharacter (Game|GetPlayerController 0)))
  (Variables|/Game/PointClick/Blueprint/PC_PointCharacter.PC_PointCharacter_C|SetCanInteract _aspc_point_character false)
  (Variables|/Game/PointClick/Blueprint/PC_PointCharacter.PC_PointCharacter_C|SetCanMove _aspc_point_character false)
  (CallFunction|ShowNoteEvent))

(fn ConstructionScript
  (|CallParentFunction))

(fn ShowNote
  (params (line :type Integer))
  (bind _note (Variables|Default|GetNote))
  (bind _lines (Utilities|Struct|BreakStruct_Note _note))
  (bind _item (Utilities|Array|Get(acopy) _lines line))
  (bind (_text _duration) (Utilities|Struct|BreakStruct_Line _item))
  (if (< line (Utilities|Array|Length _lines))
    (bind _asbp_character (Utilities|Casting|CastToBP_Character (Game|GetPlayerCharacter 0))
      (:then
        (Default|Talk _asbp_character _text _duration)
        (LocalVariables|SetNext%20Line (+ line 1)))
      (:CastFailed
        (LocalVariables|SetNext%20Line -1 :!label _label)))
    (else
      (goto _label)))
  (return (LocalVariables|GetNext%20Line) _duration))