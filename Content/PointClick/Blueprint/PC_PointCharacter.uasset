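; Player controller for a point-and-click game that moves the controlled pawn to clicked locations and holds the player's inventory.
; Left-click release, when CanMove is set, traces under the cursor and calls SimpleMoveToLocation for targets at least 120 units away; Jump input drives the character.
; Inventory functions look up items by name and mirror additions and removals to the WB_Inventory widget, which Tick finds and caches.
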(event EventTick
  (params (DeltaSeconds :type Float%20%28single-precision%29))
  (if (not (Utilities|IsValid (Variables|Default|GetInventoryUI)))
    (bind _foundwidgets (Widget|GetAllWidgetsOfClass "/Game/PointClick/UI/WB_Inventory.WB_Inventory_C" true))
    (bind _aswb_inventory (Utilities|Casting|CastToWB_Inventory (Utilities|Array|Get(acopy) _foundwidgets)))
    (Variables|Default|SetInventoryUI _aswb_inventory)))

(event Input|ActionEvents|InputActionLeftMouseClick
  (:Released
    (if (Variables|Default|GetCanMove)
      (CallFunction|MovetoLocation (.HitResult (Game|Player|GetHitResultUnderCursorbyChannel "TraceTypeQuery1" true))))))

(event Input|ActionEvents|InputActionJump
  (bind _returnvalue (Game|GetPlayerCharacter 0))
  (:Pressed
    (Character|Jump _returnvalue))
  (:Released
    (Character|StopJumping _returnvalue)))

(fn ConstructionScript)

(fn MovetoLocation
  (params (Hit%20Result :type Hit%20Result%20Structure))
  (bind _location (Collision|BreakHitResult Hit%20Result))
  (if (>= (Math|Vector|VectorLength (- (Transformation|GetActorLocation (Pawn|GetControlledPawn)) _location)) 1.2e+02)
    (AI|Navigation|SimpleMovetoLocation self _location)))

(fn GetItem
  (params (Name :type String))
  (for _array_element (Variables|Default|GetInventory)
    (if (Utilities|Enum|Equal(Enum) Name (.Name (Utilities|Struct|BreakStruct_Item _array_element)))
      (LocalVariables|SetReturnItem _array_element)
      (return (LocalVariables|GetReturnItem))))
  (return (LocalVariables|GetReturnItem)))

(fn AddItem
  (params (Item :type Struct%20Item%20Structure))
  (Utilities|Array|Add (Variables|Default|GetInventory) Item)
  (Default|AddItem (Variables|Default|GetInventoryUI) Item))

(fn GetInventory
  (return (Variables|Default|GetInventory)))

(fn RemoveItem
  (params (Item :type Struct%20Item%20Structure))
  (Utilities|Array|RemoveItem (Variables|Default|GetInventory) Item)
  (Default|RemoveItem (Variables|Default|GetInventoryUI) Item))