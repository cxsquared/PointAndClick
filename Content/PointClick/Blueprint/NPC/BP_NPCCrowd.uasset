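; BP_NPCCrowd is a crowd NPC that chatters guesses about options A, B or C.
; A self-rescheduling RandomTalk timer picks a random line at random intervals, speaking only while the player controller's InTalkingRoom flag is set.
; Interacting makes the player character voice indecision about which one to pick.
; The construction script assigns each instance a random Color.
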(event `self.ReceiveBeginPlay`
  (`parent.ReceiveBeginPlay`)
  (`KismetSystemLibrary.K2_SetTimer` null "RandomTalk" (`KismetMathLibrary.RandomFloatInRange` 0.5 5.0)))

(event `self.ReceiveActorBeginOverlap`
  (params (OtherActor :type "Actor Object Reference")))

(event `self.ReceiveTick`
  (params (DeltaSeconds :type "Float (single-precision)"))
  (`parent.ReceiveTick` 0.0))

(event `/Game/PointClick/Blueprint/Items/BP_Pickup.Interact`
  (bind _asbp_character (cast `/Game/PointCharacter/BP_Character` (`GameplayStatics.GetPlayerCharacter` 0)))
  (`/Game/PointCharacter/BP_Character.Talk` _asbp_character "I can't tell which is the right one to pick." 3.0))

(fn `RandomTalk`
  (bind _aspc_point_character (cast `/Game/PointClick/Blueprint/PC_PointCharacter` (`GameplayStatics.GetPlayerController` 0)))
  (if (`/Game/PointClick/Blueprint/PC_PointCharacter.InTalkingRoom` _aspc_point_character)
    (switch `int` (`KismetMathLibrary.RandomIntegerInRange` 0 5)
      (:`0`
        (`self.Talk` "I'm pretty sure it's A" 2.5))
      (:`1`
        (`self.Talk` "I think it's B" 2.5))
      (:`2`
        (`self.Talk` "No wait.. it's C" 2.5))
      (:`3`
        (`self.Talk` "None of them look right" 2.5))
      (:`4`
        (`self.Talk` "I'd pck A" 2.5))
      (:`5`
        (`self.Talk` "Obviously it's B" 2.5))))
  (`KismetSystemLibrary.K2_SetTimer` null "RandomTalk" (`KismetMathLibrary.RandomFloatInRange` 0.5 3.0)))

(fn `UserConstructionScript`
  (`parent.UserConstructionScript`)
  (set `self.Color` (`.ParameterValue` (break `VectorParameterValue` (make `VectorParameterValue` "None" (make `LinearColor` (`KismetMathLibrary.RandomFloat`) (`KismetMathLibrary.RandomFloat`) (`KismetMathLibrary.RandomFloat`) 1.0))))))