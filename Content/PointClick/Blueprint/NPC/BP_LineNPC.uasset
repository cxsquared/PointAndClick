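; BP_LineNPC is a dialogue NPC that offers a one-time choice of line and unlocks a linked door.
; Interact shows the options from the first statement, or says a pick was already made.
; While awaiting a response, numbered input marks the pick and records it on BP_Character, incrementing RoomsComplete.
; Only afterwards is the number checked against the response count before enabling the Door and responding.
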(event `self.ReceiveBeginPlay`
  (`parent.ReceiveBeginPlay`))

(event `self.ReceiveActorBeginOverlap`
  (params (OtherActor :type "Actor Object Reference")))

(event `self.ReceiveTick`
  (params (DeltaSeconds :type "Float (single-precision)"))
  (`parent.ReceiveTick` 0.0))

(event `self.InputHandler`
  (params (Number :type Integer))
  (if (`self.WaitingForResponse`)
    (set `self.HasPicked` true)
    (bind _asbp_character (cast `/Game/PointCharacter/BP_Character` (`GameplayStatics.GetPlayerCharacter` 0)))
    (set `/Game/PointCharacter/BP_Character.RoomsComplete` (+ (`/Game/PointCharacter/BP_Character.RoomsComplete` _asbp_character) 1) _asbp_character)
    (set `/Game/PointCharacter/BP_Character.DidTalk` true _asbp_character)
    (set `/Game/PointCharacter/BP_Character.LinePicked` Number _asbp_character)
    (if (>= (`KismetArrayLibrary.Array_Length` (`.Player_Responses_19_CD823C66468D4EB347CBFBB8EFEC7D8E` (break `/Game/PointClick/Blueprint/NPC/Struct_NPCStatement` (`KismetArrayLibrary.Array_Get` (`self.NPC_Statements`) (`self.CurrentStatment`))))) Number)
      (set `/Game/PointClick/Blueprint/Items/BP_LineDoor.CanGo` true (`self.Door`))
      (`self.Respond` Number))))

(event `/Game/PointClick/Blueprint/Items/BP_Pickup.Interact`
  (if (`self.HasPicked`)
    (`self.Talk` "You have already picked" 2.5)
    (else
      (set `self.CurrentStatment` 0)
      (`self.ShowOptions`))))

(fn `UserConstructionScript`
  (`parent.UserConstructionScript`))