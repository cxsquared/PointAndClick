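; Point-and-click NPC actor that shows a floating speech line ("Hi I'm Bob!") when interacted with.
; BeginPlay creates a hidden WB_PlayerText widget in the viewport.
; Tick projects the NPC component's world location to screen space and offsets the widget to keep it above the character.
; Talk sets and shows the text, then a named timer calls ClearText to blank and hide it.
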(event `self.ReceiveBeginPlay`
  (bind _returnvalue (`|CreateWidget` "/Game/PointClick/UI/WB_PlayerText.WB_PlayerText_C"))
  (bind _output_get (set `self.TalkWidget` _returnvalue))
  (`UserWidget.AddToViewport` _output_get 0)
  (`Widget.SetVisibility` _output_get "Hidden")
  (`UserWidget.SetDesiredSizeInViewport` _output_get (500.0 200.0)))

(event `self.ReceiveActorBeginOverlap`
  (params (OtherActor :type "Actor Object Reference")))

(event `self.ReceiveTick`
  (params (DeltaSeconds :type "Float (single-precision)"))
  (`parent.ReceiveTick` 0.0)
  (`self.UpdatedText`))

(event `self.Interact`
  (`self.Talk` "Hi I'm Bob!" 2.5))

(fn `ClearText`
  (bind _talkwidget (`self.TalkWidget`))
  (`/Game/PointClick/UI/WB_PlayerText.SetText` _talkwidget "")
  (`Widget.SetVisibility` _talkwidget "Hidden"))

(fn `Talk`
  (params (Text :type String) (Time :type "Float (double-precision)"))
  (`/Game/PointClick/UI/WB_PlayerText.SetText` (`self.TalkWidget`) Text)
  (`KismetSystemLibrary.K2_SetTimer` null "ClearText" Time)
  (`Widget.SetVisibility` (`self.TalkWidget`) "Visible"))

(fn `UpdatedText`
  (`UserWidget.SetPositionInViewport` (`self.TalkWidget`) (- (`WidgetLayoutLibrary.ProjectWorldLocationToWidgetPosition` (`GameplayStatics.GetPlayerController` 0) (`SceneComponent.K2_GetComponentLocation` (`self.NPC`))) (250.0 200.0)) false))

(fn `UserConstructionScript`
  (`parent.UserConstructionScript`))