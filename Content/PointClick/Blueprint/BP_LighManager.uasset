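; Light puzzle manager for a point-and-click game: switches toggle five lights until all are lit, revealing a key.
; FlipSwitch toggles a light and its two neighbours in a wrapping ring, updates a try-counter widget, then calls CheckLights.
; CheckLights counts leading lit lights without resetting the total between calls.
; At five it locks the puzzle, plays the key Matinee, enables key collision and triggers a character line.
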(event EventBeginPlay
  (Collision|SetCollisionEnabled (Variables|/Game/PointClick/Blueprint/Items/BP_Pickup.BP_Pickup_C|GetBox (Variables|Default|GetKey)) "NoCollision")
  (CallFunction|UpdateNumber))

(event Collision|EventActorBeginOverlap
  (params (OtherActor :type Actor%20Object%20Reference)))

(event EventTick
  (params (DeltaSeconds :type Float%20%28single-precision%29)))

(fn ConstructionScript)

(fn FlipSwitch
  (params (SwitchNumber :type Integer))
  (bind _lights (Variables|Default|GetLights))
  (if (not (Variables|Default|GetIsDone))
    (Variables|Default|SetNumberOfTries (+ (Variables|Default|GetNumberOfTries) 1))
    (CallFunction|UpdateNumber)
    (switch int SwitchNumber
      (:0
        (Utilities|FlowControl|Sequence
          (:then_0
            (Rendering|ToggleVisibility (Variables|/Script/Engine.Light|GetLightComponent (Utilities|Array|Get(acopy) _lights)) true :!label _label))
          (:then_1
            (Rendering|ToggleVisibility (Variables|/Script/Engine.Light|GetLightComponent (Utilities|Array|Get(acopy) _lights 1)) true :!label _label_2))
          (:then_2
            (Rendering|ToggleVisibility (Variables|/Script/Engine.Light|GetLightComponent (Utilities|Array|Get(acopy) _lights 4)) true :!label _label_3))
          (:then_3
            (CallFunction|CheckLights :!label _label_4))))
      (:1
        (Utilities|FlowControl|Sequence
          (:then_0
            (goto _label))
          (:then_1
            (goto _label_2))
          (:then_2
            (Rendering|ToggleVisibility (Variables|/Script/Engine.Light|GetLightComponent (Utilities|Array|Get(acopy) _lights 2)) true :!label _label_5))
          (:then_3
            (goto _label_4))))
      (:2
        (Utilities|FlowControl|Sequence
          (:then_0
            (goto _label_2))
          (:then_1
            (goto _label_5))
          (:then_2
            (Rendering|ToggleVisibility (Variables|/Script/Engine.Light|GetLightComponent (Utilities|Array|Get(acopy) _lights 3)) true :!label _label_6))
          (:then_3
            (goto _label_4))))
      (:3
        (Utilities|FlowControl|Sequence
          (:then_0
            (goto _label_5))
          (:then_1
            (goto _label_6))
          (:then_2
            (goto _label_3))
          (:then_3
            (goto _label_4))))
      (:4
        (Utilities|FlowControl|Sequence
          (:then_0
            (goto _label_6))
          (:then_1
            (goto _label_3))
          (:then_2
            (goto _label))
          (:then_3
            (goto _label_4)))))))

(fn CheckLights
  (bind _array_element (Utilities|Array|ForEachLoopwithBreak (Variables|Default|GetLights) :!label _label)
    (:LoopBody
      (if (Rendering|IsVisible (Variables|/Script/Engine.Light|GetLightComponent _array_element))
        (LocalVariables|SetNumOfLightsDone (+ 1 (LocalVariables|GetNumOfLightsDone)))
        (else
          (goto _label Break))))
    (:Completed
      (if (>= (LocalVariables|GetNumOfLightsDone) 5)
        (Variables|Default|SetIsDone true)
        (Audio|Components|Audio|Play (Variables|Default|GetKeyMatinee))
        (Collision|SetCollisionEnabled (Variables|/Game/PointClick/Blueprint/Items/BP_Pickup.BP_Pickup_C|GetBox (Variables|Default|GetKey)) "QueryAndPhysics")
        (bind _asbp_character (Utilities|Casting|CastToBP_Character (Game|GetPlayerCharacter 0)))
        (Default|Talk _asbp_character "I think I figured it out. Now where's that key?" 3.0)))))

(fn UpdateNumber
  (bind _aswb_counter (Utilities|Casting|CastToWB_Counter (UserInterface|GetUserWidgetObject (Variables|Default|GetWidget))))
  (Rendering|Components|TextRender|SetText (Variables|/Game/PointClick/UI/WB_Counter.WB_Counter_C|GetTextBlock_6 _aswb_counter) (Utilities|Text|ToText(Integer) (Variables|Default|GetNumberOfTries))))